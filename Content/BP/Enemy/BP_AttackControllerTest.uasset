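; BP_AttackControllerTest is a test actor in the Enemy folder that bobs vertically around its spawn point; it contains no attack logic.
; BeginPlay caches the starting location, and Tick offsets its Z with a sine of time since creation, leaving X and Y fixed.
; Each tick also prints that elapsed time on screen as a keyed debug string.
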(event `self.ReceiveBeginPlay`
  (set `self.Init pos` (`self.K2_GetActorLocation`)))

(event `self.ReceiveTick`
  (params (DeltaSeconds :type "Float (single-precision)"))
  (bind _returnvalue (`self.GetGameTimeSinceCreation`))
  (bind (_init_pos_x _init_pos_y _init_pos_z) (`KismetMathLibrary.BreakVector` (`self.Init pos`)))
  (`KismetSystemLibrary.PrintString` (`KismetStringLibrary.Conv_DoubleToString` _returnvalue) true true (struct :`G` 0.66 :`B` 1.0 :`A` 1.0) 0.0 "50")
  (`self.K2_SetActorLocation` (`KismetMathLibrary.MakeVector` _init_pos_x _init_pos_y (+ _init_pos_z (* (`KismetMathLibrary.Sin` _returnvalue) 100.0)))))

(fn `UserConstructionScript`)