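; BP_Attacker is an enemy Blueprint that spawns an attack collision actor aimed toward the player.
; Its AttackCollision event takes the normalized direction from itself to player character 0 and spawns a BoxColl_Test at a fixed distance along it.
; The spawn transform is built from that location alone, and the construction script is empty.
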(event `self.AttackCollision`
  (params (InValue :type "Float (single-precision)"))
  (`|SpawnActorFromClass` "/Game/BP/Enemy/BoxColl_Test.BoxColl_Test_C" (`KismetMathLibrary.Conv_VectorToTransform` (+ (`self.K2_GetActorLocation`) (* (`KismetMathLibrary.Normal` (- (`self.K2_GetActorLocation` (`GameplayStatics.GetPlayerCharacter` 0)) (`self.K2_GetActorLocation`))) (`KismetMathLibrary.Conv_DoubleToVector` 200.0)))) "Undefined" "MultiplyWithRoot" null null))

(fn `UserConstructionScript`)