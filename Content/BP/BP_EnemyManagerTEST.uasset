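; Test enemy manager that spawns a ring of enemies and flies them in formation around itself to attack the player.
; Two trigger spheres advance a status: the first spawns the evenly spaced ring, the second starts the configured attack type.
; Tick orbits enemies around the forward axis, or around the up axis with sine-varied radius and height, facing each at the player.
; During attacks, the manager follows the player beyond a boundary distance.
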(event `self.ReceiveBeginPlay`
  ;[1 1 1] begin
  (`|ExecutionSequence`
    (:`then_0`
      ;;[1 1 1] init angleInterval
      (set `self.angleInterval` (`KismetMathLibrary.SafeDivide` 360.0 (`KismetMathLibrary.Conv_IntToDouble` (`self.EnemyNum`)))))
    (:`then_1`
      (set `self.Status` "NewEnumerator0"))))

(event `self.Sphere_TriggerSpawn.OnComponentBeginOverlap`
  (params (OverlappedComponent :type "PrimitiveComponent Object Reference") (OtherActor :type "Actor Object Reference") (OtherComp :type "PrimitiveComponent Object Reference") (OtherBodyIndex :type Integer) (bFromSweep :type Boolean) (SweepResult :type "HitResult Structure (by ref)"))
  ;[1 1 1] spawn trigger
  (switch `/Game/BP/EEnemyManagerStatus` (`self.Status`)
    (:`NewEnumerator0`
      (bind _asbp_player (cast `/Game/BP/Player/BP_Player` OtherActor))
      (set `self.SF Player` _asbp_player)
      (`self.SpawnEnemy`)
      (bind _output_get (set `self.Status` "NewEnumerator1"))
      ;;[0.016 1 0] test
      (`KismetSystemLibrary.PrintString` (`|GetEnumeratorNameAsString` _output_get)))))

(event `SpawnEnemy`
  (bind (_returnvalue_location _returnvalue_rotation _returnvalue_scale) (`KismetMathLibrary.BreakTransform` (`self.GetTransform`)))
  ;[1 1 1] Spawn
  ;;[1 1 1] null check
  (`/Engine/EditorBlueprintResources/StandardMacros.IsValid` (`self.SF Player`)
    (:`Is Valid`
      ;;[1 1 1] spawn loop
      (for _index (range (`self.EnemyNum`))
        (bind _returnvalue (`|SpawnActorFromClass` (`self.enemyType`) (`KismetMathLibrary.MakeTransform` (`self.Move Around Forward Vector` _index) _returnvalue_rotation _returnvalue_scale) "AdjustIfPossibleButDontSpawnIfColliding" "MultiplyWithRoot" null null))
        ;;[1 1 1] add to array
        (`KismetArrayLibrary.Array_AddUnique` (`self.SF EnemyBase`) _returnvalue)))))

(event `self.Sphere_TriggerAttack.OnComponentBeginOverlap`
  (params (OverlappedComponent :type "PrimitiveComponent Object Reference") (OtherActor :type "Actor Object Reference") (OtherComp :type "PrimitiveComponent Object Reference") (OtherBodyIndex :type Integer) (bFromSweep :type Boolean) (SweepResult :type "HitResult Structure (by ref)"))
  ;[1 1 1] attack trigger
  (switch `/Game/BP/EEnemyManagerStatus` (`self.Status`)
    (:`NewEnumerator1`
      (bind _asbp_player (cast `/Game/BP/Player/BP_Player` OtherActor))
      (set `self.SF Player` _asbp_player)
      ;;[0 0.03912 1] debug
      (bind _output_get (set `self.Status` (`self.AttakType`)))
      ;;[0.016 1 0] test
      (`KismetSystemLibrary.PrintString` (`|GetEnumeratorNameAsString` _output_get) true false (struct :`R` 0.614583 :`B` 0.373163 :`A` 1.0)))))

(event `UpdateAttackNormal`
  (bind _sf_enemybase (`self.SF EnemyBase`))
  ;[1 1 1] attack1 : rotate
  ;;[1 1 1] rotate element
  (for (_array_element _array_index) _sf_enemybase
    (`/Engine/EditorBlueprintResources/StandardMacros.IsValid` _array_element
      (:`Is Valid`
        (`|ExecutionSequence`
          (:`then_0`
            (`self.K2_SetActorLocation` _array_element (`self.Move Around Forward Vector` _array_index) false false))
          (:`then_1`
            (`self.K2_SetActorRotation` _array_element (`KismetMathLibrary.FindLookAtRotation` (`self.K2_GetActorLocation` _array_element) (`self.K2_GetActorLocation` (`self.SF Player`))) false))))
      (:`Is Not Valid`
        (`KismetArrayLibrary.Array_RemoveItem` _sf_enemybase _array_element)))))

(event `self.ReceiveTick`
  (params (DeltaSeconds :type "Float (single-precision)"))
  ;[1 1 1] update location and orientation
  (`/Engine/EditorBlueprintResources/StandardMacros.IsValid` (`self.SF Player`)
    (:`Is Valid`
      (`|ExecutionSequence`
        (:`then_0`
          ;;[0.005 1 0] test
          (if (> (`KismetMathLibrary.Conv_ByteToInt` (`self.Status`)) 1)
            (`self.Track Player`)))
        (:`then_1`
          (switch `/Game/BP/EEnemyManagerStatus` (`self.Status`)
            (:`NewEnumerator2`
              (`self.UpdateAttackNormal`))
            (:`NewEnumerator3`
              (`self.UpdateAttack2`))))))))

(event `UpdateAttack2`
  (bind _sf_enemybase (`self.SF EnemyBase`))
  ;[1 1 1] attack2
  ;;[1 1 1] rotate element
  (for (_array_element _array_index) _sf_enemybase
    (`/Engine/EditorBlueprintResources/StandardMacros.IsValid` _array_element
      (:`Is Valid`
        (`|ExecutionSequence`
          (:`then_0`
            (`self.K2_SetActorLocation` _array_element (`self.Move Around Up Vector` _array_index) false false))
          (:`then_1`
            (`self.K2_SetActorRotation` _array_element (`KismetMathLibrary.FindLookAtRotation` (`self.K2_GetActorLocation` _array_element) (`self.K2_GetActorLocation` (`self.SF Player`))) false))))
      (:`Is Not Valid`
        (`KismetArrayLibrary.Array_RemoveItem` _sf_enemybase _array_element)))))

(fn `Move Around Forward Vector`
  (params (index :type Integer))
  (returns (location :type "Vector Structure"))
  (return (+ (`self.K2_GetActorLocation`) (* (`KismetMathLibrary.RotateAngleAxis` (`self.GetActorUpVector`) (+ (`KismetMathLibrary.Conv_IntToDouble` (* (`self.angleInterval`) index)) (mod (* (`self.GetGameTimeSinceCreation`) (`self.elementRotateSpeed`)) 360.0)) (`self.GetActorForwardVector`)) (`self.offsetFromCenter`)))))

(fn `Move Around Up Vector`
  (params (index :type Integer))
  (returns (location :type "Vector Structure"))
  (bind _returnvalue (`KismetMathLibrary.Conv_IntToDouble` (* (`self.angleInterval`) index)))
  (bind _returnvalue_2 (mod (+ _returnvalue (* (`self.GetGameTimeSinceCreation`) 120.0)) 360.0))
  (bind _returnvalue_3 (`KismetMathLibrary.DegSin` _returnvalue_2))
  (bind _returnvalue_4 (+ (`self.offsetFromCenter`) (* 300.0 _returnvalue_3)))
  (return (+ (+ (`self.K2_GetActorLocation`) (* (`KismetMathLibrary.RotateAngleAxis` (`self.GetActorForwardVector`) (+ _returnvalue _returnvalue_2) (`self.GetActorUpVector`)) _returnvalue_4)) (* (`self.GetActorUpVector`) (* _returnvalue_4 _returnvalue_3)))))

(fn `Track Player`
  (bind _returnvalue (`KismetMathLibrary.FindLookAtRotation` (`self.K2_GetActorLocation`) (`self.K2_GetActorLocation` (`self.SF Player`))))
  ;[1 1 1] distance check
  (if (> (`KismetMathLibrary.Vector_Distance` (`self.K2_GetActorLocation`) (`self.K2_GetActorLocation` (`self.SF Player`))) (`self.trackDistanceBoundary`))
    ;[1 1 1] track
    (`self.K2_SetActorRotation` _returnvalue)
    (`self.K2_AddActorWorldOffset` (`KismetMathLibrary.Conv_RotatorToVector` (* _returnvalue (`self.managerMoveSpeed`))))))

(fn `UserConstructionScript`)