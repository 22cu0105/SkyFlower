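; Test lock-on marker actor that displays a lock-on indicator through its WidgetON widget component.
; SetLockOn casts the component's widget to WBP_LockOn_UI_TEST and forwards the flag to it, while SetVisibility shows or hides the component itself.
; BeginPlay and Tick are empty; leftover test logic for moving the actor to the player's location is disconnected and never runs.
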(event `self.ReceiveBeginPlay`)

(event `self.ReceiveTick`
  (params (DeltaSeconds :type "Float (single-precision)")))

(event `SetLockOn`
  (params (IsVisible :type "ESlateVisibility Enum" :default "Visible"))
  ;[1 1 1] Comment
  (bind _aswbp_lock_on_ui_test (cast `/Game/BP/UI/WBP_LockOn_UI_TEST` (`WidgetComponent.GetUserWidgetObject` (`self.Widget_ON`))))
  (`/Game/BP/UI/WBP_LockOn_UI_TEST.SetLockOn` _aswbp_lock_on_ui_test IsVisible))

(event `SetVisibility`
  (params (IsVisible :type Boolean))
  ;[1 1 1] Comment
  (`SceneComponent.SetVisibility` (`self.Widget_ON`) IsVisible false))

(fn `UserConstructionScript`)