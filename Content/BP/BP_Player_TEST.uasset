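; Test player Blueprint prototyping enemy lock-on and a homing magic-ball attack, with debug prints.
; Tick traces along the camera-to-player direction for TargetEnemy, moves the BP_LockOnTEST icon onto it, drops wide-angle targets and sets lock display by character state.
; F12 toggles lock display; F10, marked deprecated, spawns a ring of homing balls shared round-robin among enemies near the target.
; Older attack, montage and broom code remains unwired.
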(event `self.ReceiveBeginPlay`
  ;[1 1 1] spawn lock icon
  (bind _returnvalue (`|SpawnActorFromClass` "/Game/BP/BP_LockOnTEST.BP_LockOnTEST_C" (`self.GetTransform`) "AlwaysSpawn" "MultiplyWithRoot" null null))
  (set `self.BP LockOn` _returnvalue))

(event `InputAction|TEST_F12`
  (params (Key :type "Key Structure"))
  (bind _bp_lockon (`self.BP LockOn`))
  (:`Pressed`
    ;[1 1 1] change LOCK status
    (bind _output_get (set `self.IsLOCK` (not (`self.IsLOCK`))))
    (if _output_get
      (`/Game/BP/BP_LockOnTEST.SetLockOn` _bp_lockon "Visible")
      (else
        (`/Game/BP/BP_LockOnTEST.SetLockOn` _bp_lockon "Hidden")))))

(event `InputAction|TEST_F10`
  (params (Key :type "Key Structure")))

(event `self.ReceiveTick`
  (params (DeltaSeconds :type "Float (single-precision)"))
  (bind _bp_lockon (`self.BP LockOn`))
  (bind _targetenemy (`self.TargetEnemy`))
  ;[1 1 1] show/hide Lock icon
  (`/Game/BP/BP_LockOnTEST.SetVisibility` (`self.BP LockOn`) (`KismetSystemLibrary.IsValid` (`self.TargetEnemy`)))
  (`self.RaycastForTarget`)
  ;[1 1 1] set Lock icon location
  (`/Engine/EditorBlueprintResources/StandardMacros.IsValid` _targetenemy
    (:`Is Valid`
      (`self.K2_SetActorLocation` (`self.BP LockOn`) (`self.K2_GetActorLocation` _targetenemy) false false)
      (`self.IsTargetOutOfViewport`)
      ;[1 0.05611 0] Comment
      (bind _returnvalue (`self.GetCharacterState`))
      (`KismetSystemLibrary.PrintString` (`|GetEnumeratorNameAsString` _returnvalue) true true (struct :`R` 0.110122 :`G` 1.0 :`B` 0.233897 :`A` 1.0) 0.0)
      (switch `ESF_CharacterState` _returnvalue
        (:`Normal`
          (`/Game/BP/BP_LockOnTEST.SetLockOn` _bp_lockon "Hidden" :!label _label))
        (:`ShortRangeAttack`
          (`/Game/BP/BP_LockOnTEST.SetLockOn` _bp_lockon "Visible"))
        (:`LongRangeAttack`
          (goto _label))))
    (:`Is Not Valid`
      (`KismetSystemLibrary.PrintString` "Hello" true true (struct :`R` 1.0 :`G` 0.321636 :`B` 0.361449 :`A` 1.0) 0.0))))

(event `RaycastForTarget`
  ;[1 1 1] Comment
  (bind _returnvalue (`GameplayStatics.GetActorOfClass` "/Game/BP/Camera/BP_MainCamera.BP_MainCamera_C"))
  (bind _outhit (`KismetSystemLibrary.LineTraceSingle` :`Start` (`self.K2_GetActorLocation`) :`End` (* (- (`self.K2_GetActorLocation`) (`SceneComponent.K2_GetComponentLocation` (`SF_MainCamera.CameraComponent` _returnvalue))) (`self.raycastLength`)) :`TraceChannel` "TraceTypeQuery2" :`DrawTime` 1.0))
  (`KismetSystemLibrary.PrintString` (`KismetSystemLibrary.GetDisplayName` (`.HitActor` (`GameplayStatics.BreakHitResult` _outhit))) true true (struct :`G` 0.66 :`B` 1.0 :`A` 1.0) 0.0)
  (bind _assf_enemy_base (cast `SF_EnemyBase` (`.HitActor` (`GameplayStatics.BreakHitResult` _outhit))))
  (set `self.TargetEnemy` _assf_enemy_base))

(event `IsTargetOutOfViewport`
  (bind _returnvalue (`GameplayStatics.GetActorOfClass` "/Game/BP/Camera/BP_MainCamera.BP_MainCamera_C"))
  (if (> (`KismetMathLibrary.DegAcos` (`KismetMathLibrary.Dot_VectorVector` (`KismetMathLibrary.Vector_NormalUnsafe` (- (`self.K2_GetActorLocation` (`self.BP LockOn`)) (`self.K2_GetActorLocation`))) (`KismetMathLibrary.Vector_NormalUnsafe` (- (`self.K2_GetActorLocation`) (`SceneComponent.K2_GetComponentLocation` (`SF_MainCamera.CameraComponent` _returnvalue)))))) 60.0)
    (set `self.TargetEnemy` null)
    (`KismetSystemLibrary.PrintString` "CLEAR TARGET" true true (struct :`G` 0.66 :`B` 1.0 :`A` 1.0) 10.0)))

(event `InputAction|TEST_F10`
  (params (Key :type "Key Structure"))
  (bind _targetenemy (`self.TargetEnemy`))
  (bind _returnvalue (`KismetArrayLibrary.Array_Length` (`self.Out Actors`)))
  (bind _magicballnumber (`SF_AttackInput.magicballNumber` (`self.AttackInputComponent`)))
  ;[1 1 1] Comment
  (:`Pressed`
    ;[0.5168 0 1] deprecated - homing attack
    ;;[1 1 1] Comment
    (bind _asbp_game_mode_testempty_level (cast `/Game/BP/BP_GameModeTESTemptyLevel` (`GameplayStatics.GetGameMode`))
      (:`then`
        (bind _asbp_player_test (cast `/Game/BP/BP_Player_TEST` (`GameplayStatics.GetPlayerPawn` 0))
          (:`then`
            (if (`KismetSystemLibrary.IsValid` _targetenemy)
              ;;[1 1 1] make enemy list
              (bind _outactors (`KismetSystemLibrary.SphereOverlapActors` (`self.K2_GetActorLocation` _targetenemy) 1200.0 (`self.Object Types`) "/Script/SkyFlower.SF_EnemyBase"))
              (set `self.Out Actors` _outactors)
              (bind _output_get (set `self.homingBallNum` (- (`KismetArrayLibrary.Array_Length` _outactors) 1)))
              (`KismetSystemLibrary.PrintString` (`KismetStringLibrary.Conv_IntToString` _output_get))
              (else
                ;;[1 1 1] no target, default
                (set `self.homingBallNum` (- _magicballnumber 1))))
            (for _index (range (+ _magicballnumber 1))
              (bind _returnvalue_2 (`self.GetActorForwardVector` _asbp_player_test))
              (bind _returnvalue_3 (`|SpawnActorFromClass` "/Game/BP/Weapon/BP_HomingMagicball.BP_HomingMagicball_C" (`KismetMathLibrary.MakeTransform` (`self.K2_GetActorLocation` _asbp_player_test) (`KismetMathLibrary.Conv_VectorToRotator` (+ (`KismetMathLibrary.RotateAngleAxis` (+ _returnvalue_2 (`KismetMathLibrary.MakeRotator` 0.0 90.0)) (* (/ (`SF_AttackInput.angleStep` (`self.AttackInputComponent`)) _magicballnumber) _index) _returnvalue_2) (* (`SceneComponent.GetForwardVector` (`SF_MainCamera.CameraComponent` (`SF_GameMode.GetMainCamera` _asbp_game_mode_testempty_level))) (-5.0 -5.0 -5.0))))) "Undefined" "MultiplyWithRoot" null null))
              (if (> _returnvalue 0)
                (bind _assf_enemy_base (cast `SF_EnemyBase` (`|GetArrayItem` (`self.Out Actors`) (mod _index _returnvalue))))
                (`SF_HomingMagicball.InitTarget` _returnvalue_3 _assf_enemy_base)))
            (`KismetArrayLibrary.Array_Clear` (`self.Out Actors`)))
          (:`CastFailed`
            (`KismetSystemLibrary.PrintString` "cast failed" :!label _label_2))))
      (:`CastFailed`
        (goto _label_2)))))

(fn `UserConstructionScript`)