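; BP_Player is the player Blueprint, holding a test input that fires a volley of homing magic balls.
; Pressing TEST spawns BP_HomingballTEST actors at the player's location, with the count and angle step taken from AttackInputComponent.
; Each launch direction is fanned around the player's forward axis, then biased against the main camera's forward vector, obtained through BP_GameMode.
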(event `InputAction|TEST`
  (params (Key :type "Key Structure"))
  (bind _attackinputcomponent (`self.AttackInputComponent`))
  (:`Pressed`
    (bind _asbp_game_mode (cast `/Game/BP_GameMode` (`GameplayStatics.GetGameMode`)))
    (bind _asbp_player (cast `/Game/BP/Player/BP_Player` (`GameplayStatics.GetPlayerPawn` 0)))
    (for _index (range (`SF_AttackInput.magicballNumber` (`self.AttackInputComponent`)))
      (bind _returnvalue (`self.GetActorForwardVector` _asbp_player))
      (`|SpawnActorFromClass` "/Game/BP/BP_HomingballTEST.BP_HomingballTEST_C" (`KismetMathLibrary.MakeTransform` (`self.K2_GetActorLocation` _asbp_player) (`KismetMathLibrary.Conv_VectorToRotator` (+ (`KismetMathLibrary.RotateAngleAxis` (+ _returnvalue (`KismetMathLibrary.MakeRotator` 0.0 90.0)) (* (/ (`SF_AttackInput.angleStep` _attackinputcomponent) (`SF_AttackInput.magicballNumber` _attackinputcomponent)) _index) _returnvalue) (* (`SceneComponent.GetForwardVector` (`SF_MainCamera.CameraComponent` (`SF_GameMode.GetMainCamera` _asbp_game_mode))) (-5.0 -5.0 -5.0))))) "Undefined" "MultiplyWithRoot" null null))))

(fn `UserConstructionScript`)