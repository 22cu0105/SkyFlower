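; BP_HomingballTEST is a test homing projectile that chases an enemy.
; On BeginPlay it takes the first BP_EnemyMiddle actor in the level and sets its root component as the movement component's homing target.
; Each tick it raises the homing acceleration by a fixed step up to a cap, independent of delta time, so the pull toward the target ramps up.
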(event `self.ReceiveBeginPlay`
  ;[1 1 1] find a target
  (bind _outactors (`GameplayStatics.GetAllActorsOfClass` "/Game/BP/Enemy/BP_EnemyMiddle.BP_EnemyMiddle_C"))
  (for (_array_element _array_index) _outactors
    (if (== _array_index 0)
      (set `ProjectileMovementComponent.HomingTargetComponent` (`Actor.RootComponent` _array_element) (`self.MovementComp`)))))

(event `self.ReceiveTick`
  (params (DeltaSeconds :type "Float (single-precision)"))
  ;[1 1 1] speed up
  (bind _output_get (set `self.HomingAccelerate` (`KismetMathLibrary.FClamp` (+ (`self.HomingAccelerate`) 100.0) 0.0 3000.0)))
  (set `ProjectileMovementComponent.HomingAccelerationMagnitude` _output_get (`self.MovementComp`)))

(fn `UserConstructionScript`)